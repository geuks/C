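; PC_Lobby is the lobby player controller that brings up the lobby menu for its player.
; On BeginPlay, the authority side waits briefly for the client, then calls ClientShowMenu.
; That event creates the W_LobbyMenu widget for this controller, stores it on both the controller and the GI_Lobby game instance, then adds it to the player screen.
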(event `self.ReceiveBeginPlay`
  (`/Engine/EditorBlueprintResources/ActorMacros.Switch Has Authority`
    (:`Authority`
      ;[1 1 1] En attente du Client
      (`KismetSystemLibrary.Delay` 0.5)
      (`self.ClientShowMenu`))))

(event `ClientShowMenu`
  (bind _returnvalue (`|CreateWidget` "/Game/Lobby/W_LobbyMenu.W_LobbyMenu_C" self))
  (bind _output_get (set `self.LobbyMenu` _returnvalue))
  (bind _asgi_lobby (cast `/Game/Lobby/GI_Lobby` (`GameplayStatics.GetGameInstance`)))
  (set `/Game/Lobby/GI_Lobby.W_Menu` _output_get _asgi_lobby)
  (`UserWidget.AddToPlayerScreen` _output_get 0))

(fn `UserConstructionScript`)