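; PC_Main is a player controller that turns a Fire press into a direction stored on the player's state.
; It deprojects the mouse position to a world direction and passes it to ReplicateMove, which writes it to PS_Main's Direction only on authority.
; BeginPlay is empty, and the nodes that create and show the HUD_Player widget are left unconnected.
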(event `ReplicateMove`
  (params (Target :type "PlayerController Object Reference") (NewParam :type "Vector Structure"))
  (`/Engine/EditorBlueprintResources/ActorMacros.Switch Has Authority`
    (:`Authority`
      (bind _asps_main (cast `/Game/Controllers/PS_Main` (`self.PlayerState`)))
      (set `/Game/Controllers/PS_Main.Direction` NewParam _asps_main))))

(event `InputAction|Fire` :consume false
  (params (Key :type "Key Structure"))
  (:`Pressed`
    (`self.ReplicateMove` self (`.WorldDirection` (`self.DeprojectMousePositionToWorld`)))))

(event `self.ReceiveBeginPlay`)

(fn `UserConstructionScript`)