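; BP_Bullets is a projectile actor that damages 2D player characters on contact.
; Its sphere overlap checks the other actor's class name, then subtracts a fixed amount from that player's Life, updates its HUD health bar and destroys the bullet.
; Any other overlap also destroys it, and a timed delay on BeginPlay removes it if player 0 casts to BPC2d_Players.
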(event `self.ReceiveBeginPlay`
  (bind _asbpc2d_players (cast `/Game/Controllers/BPC2d_Players` (`GameplayStatics.GetPlayerCharacter` 0)))
  (set `self.Player` _asbpc2d_players)
  (`KismetSystemLibrary.Delay` 6.0)
  (`self.K2_DestroyActor`))

(event `RemoveLife`
  (params (Target :type "/Game/Controllers/BPC2d_Players Object Reference"))
  (bind _output_get (set `/Game/Controllers/BPC2d_Players.Life` (- (`/Game/Controllers/BPC2d_Players.Life` Target) 10.0) Target))
  (bind _returnvalue (* _output_get 0.01))
  (`ProgressBar.SetPercent` (`/Game/HUD/HUD_Player.ProgressBar_111` (`/Game/Controllers/BPC2d_Players.HUDPlayer` Target)) _returnvalue)
  (`KismetSystemLibrary.PrintString` (`KismetStringLibrary.Conv_DoubleToString` _returnvalue))
  (`self.K2_DestroyActor`))

(event `self.Sphere.OnComponentBeginOverlap`
  (params (OverlappedComponent :type "PrimitiveComponent Object Reference") (OtherActor :type "Actor Object Reference") (OtherComp :type "PrimitiveComponent Object Reference") (OtherBodyIndex :type Integer) (bFromSweep :type Boolean) (SweepResult :type "HitResult Structure (by ref)"))
  (if (`KismetStringLibrary.EqualEqual_StrStr` (`KismetSystemLibrary.GetClassDisplayName` (`GameplayStatics.GetObjectClass` OtherActor)) "BPC2d_Players_C")
    (bind _asbpc2d_players (cast `/Game/Controllers/BPC2d_Players` OtherActor))
    (`self.RemoveLife` _asbpc2d_players)
    (else
      (`self.K2_DestroyActor`))))

(fn `UserConstructionScript`)