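; BP_Speed is a speed boost trigger that temporarily doubles the player's walk speed.
; Its collision component's begin overlap passes the actor to serveur_collision, which compares display names with player character 0 and casts that character to BPC2d_Players.
; An IsSpeed flag blocks retriggering while boosted.
; After a short delay, it sets walk speed to the VMaxspeed variable, which this file never assigns, and clears the flag.
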(event `serveur_collision`
  (params (Trigger :type "Actor Object Reference"))
  (bind _returnvalue (`GameplayStatics.GetPlayerCharacter` 0))
  (if (`KismetStringLibrary.EqualEqual_StrStr` (`KismetSystemLibrary.GetDisplayName` _returnvalue) (`KismetSystemLibrary.GetDisplayName` Trigger))
    (if (not (`self.IsSpeed`))
      (bind _asbpc2d_players (cast `/Game/Controllers/BPC2d_Players` _returnvalue))
      (set `self.IsSpeed` true)
      (bind _charactermovement (`Character.CharacterMovement` _asbpc2d_players))
      (bind _returnvalue_2 (`MovementComponent.GetMaxSpeed` _charactermovement))
      (`KismetSystemLibrary.PrintString` (`KismetStringLibrary.Conv_DoubleToString` _returnvalue_2))
      (set `CharacterMovementComponent.MaxWalkSpeed` (* _returnvalue_2 2.0) _charactermovement)
      (`KismetSystemLibrary.Delay` 2.0)
      (set `CharacterMovementComponent.MaxWalkSpeed` (`self.VMaxspeed`) _charactermovement)
      (set `self.IsSpeed` false))))

(event `self.CollisionComp.OnComponentBeginOverlap`
  (params (OverlappedComponent :type "PrimitiveComponent Object Reference") (OtherActor :type "Actor Object Reference") (OtherComp :type "PrimitiveComponent Object Reference") (OtherBodyIndex :type Integer) (bFromSweep :type Boolean) (SweepResult :type "HitResult Structure (by ref)"))
  (`self.serveur_collision` OtherActor))

(fn `UserConstructionScript`)